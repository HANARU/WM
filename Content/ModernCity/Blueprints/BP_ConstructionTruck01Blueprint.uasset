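; Drivable construction dump truck pawn with throttle, steering, handbrake and a spring-arm camera.
; Q and E raise or lower the dumpster and back door together; Tick eases both values in the mesh's anim Blueprint with FInterpTo.
; The construction script applies materials per slot and configures two spotlights.
; BeginPlay runs a PhysX collision debug command, and both look axes share one node driving pitch and yaw together.
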(event `self.ReceiveBeginPlay`
  (`KismetSystemLibrary.ExecuteConsoleCommand` "PXVIS COLLISION" null)
  (bind _asab_ct01anim_blur_print (cast `` (`SkeletalMeshComponent.GetAnimInstance` (`self.Mesh`))))
  (set `self.CT01AnimBP` _asab_ct01anim_blur_print))

(event `Key|Q`
  (params (Key :type "Key Structure"))
  (:`Pressed`
    (set `self.WantDumpsterGoUp` true)
    (set `self.WantBackDoorOpen` true)))

(event `Key|E`
  (params (Key :type "Key Structure"))
  (:`Pressed`
    (set `self.WantDumpsterGoUp` false)
    (set `self.WantBackDoorOpen` false)))

(event `InputAxis|Throttle`
  (params (AxisValue :type "Float (single-precision)"))
  (bind _vehiclemovementcomponent (`self.VehicleMovementComponent`))
  (`self.SetThrottleInput` _vehiclemovementcomponent AxisValue)
  (`self.SetBrakeInput` _vehiclemovementcomponent (`KismetMathLibrary.Conv_BoolToDouble` (== AxisValue -1.0))))

(event `InputAxis|Steer`
  (params (AxisValue :type "Float (single-precision)"))
  (`self.SetSteeringInput` (`self.VehicleMovementComponent`) AxisValue))

(event `Key|SpaceBar`
  (params (Key :type "Key Structure"))
  (bind _vehiclemovementcomponent (`self.VehicleMovementComponent`))
  (:`Pressed`
    (`self.SetHandbrakeInput` _vehiclemovementcomponent true))
  (:`Released`
    (`self.SetHandbrakeInput` _vehiclemovementcomponent false)))

(event `InputAxis|LookUp`
  (params (AxisValue :type "Float (single-precision)"))
  (`SceneComponent.K2_AddRelativeRotation` (`self.SpringArm`) (`KismetMathLibrary.MakeRotator` 0.0 AxisValue (stale `InputAxis|LookRight` AxisValue)) false false :!label _label))

(event `InputAxis|LookRight`
  (params (AxisValue :type "Float (single-precision)"))
  (goto _label))

(event `self.ReceiveTick`
  (params (DeltaSeconds :type "Float (single-precision)"))
  (bind _returnvalue (`GameplayStatics.GetWorldDeltaSeconds`))
  (bind _ct01animbp (`self.CT01AnimBP`))
  (set `/Game/ModernCity/Blueprints/BP_ConstructionTruck01Blueprint.DumpingGoingUpCT01` (`KismetMathLibrary.FInterpTo` (`/Game/ModernCity/Blueprints/BP_ConstructionTruck01Blueprint.DumpingGoingUpCT01` _ct01animbp) (`KismetMathLibrary.SelectFloat` 20.0 0.0 (`self.WantDumpsterGoUp`)) _returnvalue 0.3) _ct01animbp)
  (set `/Game/ModernCity/Blueprints/BP_ConstructionTruck01Blueprint.BackDoorOpeningCT01` (`KismetMathLibrary.FInterpTo` (`/Game/ModernCity/Blueprints/BP_ConstructionTruck01Blueprint.BackDoorOpeningCT01` _ct01animbp) (`KismetMathLibrary.SelectFloat` -60.0 0.0 (`self.WantBackDoorOpen`)) _returnvalue 0.3) _ct01animbp))

(fn `UserConstructionScript`
  (bind _mesh (`self.Mesh`))
  (bind _exterior_material (`self.Exterior Material`))
  (`PrimitiveComponent.SetMaterial` _mesh 0 _exterior_material)
  (`PrimitiveComponent.SetMaterial` _mesh 1 _exterior_material)
  (`PrimitiveComponent.SetMaterial` _mesh 2 (`self.Light Material`))
  (`PrimitiveComponent.SetMaterial` _mesh 3 (`self.Interior Material`))
  (`PrimitiveComponent.SetMaterial` _mesh 4 (`self.Wheel Material`))
  (`PrimitiveComponent.SetMaterial` _mesh 5 (`self.Hydraulic Material`))
  (`LightComponent.SetLightColor` (`self.SpotLight1`) (`self.Light Colour`) true)
  (`LightComponent.SetLightColor` (`self.SpotLight`) (`self.Light Colour`) true)
  (`LightComponent.SetIntensity` (`self.SpotLight`) (`self.Light Intensity`))
  (`LightComponent.SetIntensity` (`self.SpotLight1`) (`self.Light Intensity`)))