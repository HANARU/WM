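; BP_ctOSMain is a level-progression actor for the ctOS hacking events, caching the BP_WMInstance game instance on begin play.
; The level 1 hack attempt triggers the game instance's fourth UI event.
; The level 2 attempt fades the screen with a UI_Fade widget, waits briefly, then opens the 3_CutScene level.
; A counter event increments and prints a count, then fires the seventh UI event once it has already counted.
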(event `self.ReceiveBeginPlay`
  (bind _asbp_wminstance (cast `/Game/2_BP/BP_System/BP_WMInstance` (`GameplayStatics.GetGameInstance`)))
  (set `self.GameInstance` _asbp_wminstance))

(event `self.LV1TryHackCTOS`
  (`/Game/2_BP/BP_System/BP_WMInstance.EventUI_4th` (`self.GameInstance`)))

(event `self.LV2TryHackCTOS`
  (bind _returnvalue (`|CreateWidget` "/Game/2_BP/BP_UI/UI_Fade.UI_Fade_C"))
  (`UserWidget.AddToViewport` _returnvalue 0)
  (`UserWidget.PlayAnimation` _returnvalue (`/Game/2_BP/BP_UI/UI_Fade.FadeIn` _returnvalue) 0.0 1 "Forward" 1.0 false)
  (`KismetSystemLibrary.Delay` 1.0)
  (`GameplayStatics.OpenLevel` "3_CutScene"))

(event `/Game/2_BP/BPI_HackableEvents.Count++`
  (bind _countap (`self.CountAP`))
  (if (>= _countap 1)
    (`/Game/2_BP/BP_System/BP_WMInstance.EventUI_7th` (`self.GameInstance`))
    (else
      (bind _result (`/Engine/EditorBlueprintResources/StandardMacros.IncrementInt` _countap)
        (:`  `
          (bind _output_get (set `self.CountAP` _result))
          (`KismetSystemLibrary.PrintString` (`KismetStringLibrary.Conv_IntToString` _output_get)))))))

(fn `UserConstructionScript`)