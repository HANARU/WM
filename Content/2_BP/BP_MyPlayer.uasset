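; Player Blueprint that looks up points on nearby cover splines when C is pressed, as groundwork for a cover system.
; FindNearestSpline gathers every BP_CurveSpline actor and prints each spline's closest world-space point to the player.
; It never compares distances, so NewLocation keeps the last spline's point, which C prints again.
; MovePlayerTo is an empty stub, so the player is not moved.
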(event `self.ReceiveBeginPlay`)

(event `Key|C`
  (params (Key :type "Key Structure"))
  (:`Pressed`
    (`self.Find Nearest Spline`)
    (`KismetSystemLibrary.PrintString` (`KismetStringLibrary.Conv_VectorToString` (`self.NewLocation`)))))

(event `Find Nearest Spline`
  (bind (_returnvalue_x _returnvalue_y _returnvalue_z) (`KismetMathLibrary.BreakVector` (`self.K2_GetActorLocation`)))
  ;[1 1 1] 플레이에서 가까운 엄폐공간(Spline) 찾기
  (bind _outactors (`GameplayStatics.GetAllActorsOfClass` "/Game/2_BP/BP_CurveSpline.BP_CurveSpline_C"))
  (bind _output_get (set `self.Splines` _outactors))
  (for _array_element _output_get
    (bind (_returnvalue_x_2 _returnvalue_y_2 _returnvalue_z_2) (`KismetMathLibrary.BreakVector` (`SplineComponent.FindLocationClosestToWorldLocation` (`/Game/2_BP/BP_CurveSpline.Spline` _array_element) (`KismetMathLibrary.MakeVector` _returnvalue_x _returnvalue_y _returnvalue_z) "World")))
    (bind _output_get_2 (set `self.NewLocation` (`KismetMathLibrary.MakeVector` _returnvalue_x_2 _returnvalue_y_2 _returnvalue_z_2)))
    (`KismetSystemLibrary.PrintString` (`KismetStringLibrary.Conv_VectorToString` _output_get_2))))

(event `Move Player To`
  (params (Location :type "Vector Structure")))

(fn `UserConstructionScript`)