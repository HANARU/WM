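; BP_CCTV_Hacked is a controllable hackable CCTV camera that the player looks through to inspect other cameras, hackable objects and enemy AI, then exits back to the player.
; Interaction input drives inherited press and one-second hold functions, with progress shown on the target camera and through a dynamic material progress bar.
; Contact events cache the target and show its info widget.
; Hacking triggers a game-instance UI event; disabling clears custom-depth highlights on cameras and BP_ctOSAP actors.
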(event `self.ReceiveBeginPlay`
  (bind _returnvalue (`|CreateWidget` "/Game/2_BP/BP_UI/UI_HackedCCTVInfo.UI_HackedCCTVInfo_C"))
  (set `self.UI Hacked CCTV` _returnvalue)
  (bind _returnvalue_2 (`|CreateWidget` "/Game/2_BP/BP_UI/UI_HackedObjectInfo.UI_HackedObjectInfo_C"))
  (set `self.UI Hacked Object` _returnvalue_2)
  (bind _returnvalue_3 (`|CreateWidget` "/Game/2_BP/BP_UI/UI_HackedAIInfo.UI_HackedAIInfo_C"))
  (set `self.UI Tracked AI` _returnvalue_3))

(event `EnhancedInput|/Game/6_MISC/Input/Actions/IA_Look`
  (params (ActionValue :type "Vector2D Structure") (ElapsedSeconds :type "Float (double-precision)") (TriggeredSeconds :type "Float (double-precision)") (InputAction :type "InputAction Object Reference" :default "/Game/6_MISC/Input/Actions/IA_Look.IA_Look"))
  (:`Triggered`
    (`self.AddControllerYawInput` ActionValue_X)
    (`self.AddControllerPitchInput` (* ActionValue_Y -1.0))))

(event `EnhancedInput|/Game/6_MISC/Input/Actions/IA_Interaction`
  (params (ActionValue :type Boolean) (ElapsedSeconds :type "Float (double-precision)") (TriggeredSeconds :type "Float (double-precision)") (InputAction :type "InputAction Object Reference" :default "/Game/6_MISC/Input/Actions/IA_Interaction.IA_Interaction"))
  (bind _interactable_cctv (`self.Interactable CCTV`))
  (:`Triggered`
    (`self.InteractStart_1Sec`)
    (if (`KismetSystemLibrary.IsValid` _interactable_cctv) :!label _label
      (message `/Game/2_BP/BPI_HackableEvents.UpdateHackingProgress` _interactable_cctv (`self.InteractionTime`))))
  (:`Started`
    (`self.InteractionSinglePress`))
  (:`Completed`
    (`self.InteractEnd_1Sec`)
    (goto _label)))

(event `EnhancedInput|/Game/6_MISC/Input/Actions/IA_Back2Player`
  (params (ActionValue :type Boolean) (ElapsedSeconds :type "Float (double-precision)") (TriggeredSeconds :type "Float (double-precision)") (InputAction :type "InputAction Object Reference" :default "/Game/6_MISC/Input/Actions/IA_Back2Player.IA_Back2Player"))
  (:`Started`
    (bind _asbp_wminstance (cast `/Game/2_BP/BP_System/BP_WMInstance` (`GameplayStatics.GetGameInstance`)))
    (`self.Back2Player` (`WM_Instance.Player` _asbp_wminstance) (`GameplayStatics.GetPlayerController` 0))))

(event `/Game/2_BP/BPI_HackableEvents.UpdateHackingProgress`
  (params (`Progress Value` :type "Float (double-precision)"))
  ;[1 1 1] Update CCTV UI Progress bar
  (bind _asui_focused_interactable_actor (cast `/Game/2_BP/BP_UI/UI_FocusedInteractableActor` (`WidgetComponent.GetUserWidgetObject` (`self.InteractableWidget`))))
  (`/Engine/EditorBlueprintResources/StandardMacros.IsValid` _asui_focused_interactable_actor
    (:`Is Valid`
      (bind _progressbar (`/Game/2_BP/BP_UI/UI_FocusedInteractableActor.ProgressBar` _asui_focused_interactable_actor))
      (bind _returnvalue (`Image.GetDynamicMaterial` _progressbar))
      (`Image.SetBrushFromMaterial` _progressbar _returnvalue)
      (`MaterialInstanceDynamic.SetScalarParameterValue` _returnvalue "Progress" `Progress Value`))))

(event `self.OnInteractionCCTV`
  (params (ContactActor :type "HitResult Structure"))
  (bind _asbp_cctv_hacked (cast `/Game/2_BP/BP_CCTV_Hacked` (`.HitActor` (`GameplayStatics.BreakHitResult` ContactActor))))
  (set `self.Interactable CCTV` _asbp_cctv_hacked)
  (`UserWidget.AddToViewport` (`self.UI Hacked CCTV`) 0))

(event `self.EndInteraction`
  (`Widget.RemoveFromParent` (`self.UI Hacked CCTV`))
  (`Widget.RemoveFromParent` (`self.UI Hacked Object`))
  (`Widget.RemoveFromParent` (`self.UI Tracked AI`)))

(event `self.OnInteractionObject`
  (params (ContactActor :type "HitResult Structure"))
  (bind _ui_hacked_object (`self.UI Hacked Object`))
  (bind _ashackable_actor (cast `HackableActor` (`.HitActor` (`GameplayStatics.BreakHitResult` ContactActor))))
  (bind _output_get (set `self.Interactable Object` _ashackable_actor))
  (`/Game/2_BP/BP_UI/UI_HackedObjectInfo.Get Object Data` _ui_hacked_object (`HackableActor.Object_Num` _output_get))
  (`UserWidget.AddToViewport` _ui_hacked_object 0))

(event `self.OnInteractionAI`
  (params (ContactActor :type "HitResult Structure"))
  (bind _ui_tracked_ai (`self.UI Tracked AI`))
  (bind _asbp_enemy_base (cast `/Game/2_BP/BP_EnemyBase` (`.HitActor` (`GameplayStatics.BreakHitResult` ContactActor))))
  (bind _output_get (set `self.Tracked AI` _asbp_enemy_base))
  (`/Game/2_BP/BP_UI/UI_HackedAIInfo.Get AI Data` _ui_tracked_ai (`AI_EnemyBase.AI_Num` _output_get))
  (`UserWidget.AddToViewport` _ui_tracked_ai 0))

(event `self.OnTargetHacked`
  (bind _asbp_wminstance (cast `/Game/2_BP/BP_System/BP_WMInstance` (`GameplayStatics.GetGameInstance`)))
  (`/Game/2_BP/BP_System/BP_WMInstance.EventUI_5th` _asbp_wminstance))

(event `self.OnDisableProcess`
  (`|ExecutionSequence`
    (:`then_0`
      (bind _outactors (`GameplayStatics.GetAllActorsOfClass` "BP_CCTV_Hacked_C"))
      (for _array_element _outactors
        (`PrimitiveComponent.SetRenderCustomDepth` (`HackableActor_CCTV.CameraBody` _array_element) false)
        (`PrimitiveComponent.SetRenderCustomDepth` (`HackableActor_CCTV.CameraSupport` _array_element) false)))
    (:`then_1`
      (bind _outactors_2 (`GameplayStatics.GetAllActorsOfClass` "/Game/2_BP/BP_CTOSAP.BP_ctOSAP_C"))
      (for _array_element_2 _outactors_2
        (`PrimitiveComponent.SetRenderCustomDepth` (`HackableActor.BodyMesh` _array_element_2) false)))))

(fn `UserConstructionScript`)