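; Player character Blueprint that handles aiming, shooting, interaction, climbing and vaulting, and registers itself with the game instance on BeginPlay.
; Enhanced Input drives zoom, shoot and tap or hold interaction functions defined outside these graphs.
; A shot fired without aiming zooms in briefly, then Tick zooms out after a delay.
; Climb and vault use Motion Warping montages, with Flying mode and collision off until completion restores walking, collision and input.
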(event `self.ReceiveTick`
  (params (DeltaSeconds :type "Float (single-precision)"))
  (set `self.CurrentZoomTime` (+ DeltaSeconds (`self.CurrentZoomTime`)))
  (if (and (`self.Shooting`) (> (`self.CurrentZoomTime`) (`self.ZoomTimeFlag`)))
    (`self.ZoomOut`)
    (set `self.Shooting` false)))

(event `self.ReceiveBeginPlay`
  (bind _asbp_wminstance (cast `/Game/2_BP/BP_System/BP_WMInstance` (`GameplayStatics.GetGameInstance`)))
  (set `WM_Instance.Player` self _asbp_wminstance))

(event `ReceivePossessed_1`
  (params (NewController :type "Controller Object Reference"))
  (set `self.IsPossessing` true))

(event `ReceiveUnpossessed_1`
  (params (OldController :type "Controller Object Reference"))
  (set `self.IsPossessing` false))

(event `EnhancedInput|/Game/6_MISC/Input/Actions/IA_Interaction`
  (params (ActionValue :type Boolean) (ElapsedSeconds :type "Float (double-precision)") (TriggeredSeconds :type "Float (double-precision)") (InputAction :type "InputAction Object Reference" :default "/Game/6_MISC/Input/Actions/IA_Interaction.IA_Interaction"))
  (:`Triggered`
    (`self.InteractStart_1Sec`))
  (:`Started`
    (`self.InteractionSinglePress`))
  (:`Completed`
    (`self.InteractEnd_1Sec`)))

(event `EnhancedInput|/Game/6_MISC/Input/Actions/IA_MouseRightClick`
  (params (ActionValue :type Boolean) (ElapsedSeconds :type "Float (double-precision)") (TriggeredSeconds :type "Float (double-precision)") (InputAction :type "InputAction Object Reference" :default "/Game/6_MISC/Input/Actions/IA_MouseRightClick.IA_MouseRightClick"))
  (:`Triggered`
    (`self.ZoomIn`))
  (:`Completed`
    (`self.ZoomOut`)))

(event `EnhancedInput|/Game/6_MISC/Input/Actions/IA_MouseLeftClick`
  (params (ActionValue :type Boolean) (ElapsedSeconds :type "Float (double-precision)") (TriggeredSeconds :type "Float (double-precision)") (InputAction :type "InputAction Object Reference" :default "/Game/6_MISC/Input/Actions/IA_MouseLeftClick.IA_MouseLeftClick"))
  (:`Started`
    (if (`self.isZooming`)
      (`self.Shoot`)
      (else
        (`self.ZoomIn`)
        (set `self.CurrentZoomTime` 0.0)
        (set `self.Shooting` true)
        (`self.Shoot`)
        (set `self.isZooming` false)))))

(event `self.ClimbMotionWarp`
  (bind (_startpos_x _startpos_y _startpos_z) (`KismetMathLibrary.BreakVector` (`self.StartPos`)))
  (bind (_wallpos_x _wallpos_y) (`KismetMathLibrary.BreakVector` (`self.WallPos`)))
  ;[1 1 1] Climb Motion 정의
  (if (`self.canClimb`)
    (`CharacterMovementComponent.SetMovementMode` (`self.CharacterMovement`) "MOVE_Flying" 0)
    (`self.SetActorEnableCollision` false)
    (`MotionWarpingComponent.AddOrUpdateWarpTargetFromTransform` (`self.MotionWraping`) "attachedMotion" (`KismetMathLibrary.MakeTransform` (`KismetMathLibrary.MakeVector` _wallpos_x _wallpos_y _startpos_z)))
    (`|PlayMontage` (`self.Mesh`) "/Game/4_SK/XBot/Animations/Montage/Braced_Hang_To_Crouch_Montage.Braced_Hang_To_Crouch_Montage"
      (:`OnCompleted`
        (`CharacterMovementComponent.SetMovementMode` (`self.CharacterMovement`) "MOVE_Walking" 0)
        (`self.SetActorEnableCollision` true)
        (`self.EnableInput` (`GameplayStatics.GetPlayerController` 0))))))

(event `self.PlayStopMontage`
  (if (not (`self.isZooming`))
    (`self.PlayAnimMontage` null)))

(event `self.VaultMotionWarp`
  ;[1 1 1] Vault Motion 정의
  (`CharacterMovementComponent.SetMovementMode` (`self.CharacterMovement`) "MOVE_Flying" 0)
  (`self.SetActorEnableCollision` false)
  (`MotionWarpingComponent.AddOrUpdateWarpTargetFromTransform` (`self.MotionWraping`) "JumpPos" (`KismetMathLibrary.MakeTransform` (`self.StartPos`) (`self.K2_GetActorRotation`)))
  (`MotionWarpingComponent.AddOrUpdateWarpTargetFromTransform` (`self.MotionWraping`) "StandPos" (`KismetMathLibrary.MakeTransform` (`self.LastPos`)))
  (`|PlayMontage` (`self.Mesh`) "/Game/4_SK/XBot/Animations/Montage/Jumping_Down_Montage.Jumping_Down_Montage"
    (:`OnCompleted`
      (`CharacterMovementComponent.SetMovementMode` (`self.CharacterMovement`) "MOVE_Walking" 0)
      (`self.SetActorEnableCollision` true)
      (`self.EnableInput` (`GameplayStatics.GetPlayerController` 0)))))

(event `self.PlayShootMontage`
  (`self.PlayAnimMontage` "/Game/4_SK/XBot/Animations/Montage/Shooting_Montage.Shooting_Montage" 3.0))

(event `self.OnInteraction`
  (params (HitActor :type "HitResult Structure"))
  (`KismetSystemLibrary.PrintString` "OnInteract"))

(fn `UserConstructionScript`)