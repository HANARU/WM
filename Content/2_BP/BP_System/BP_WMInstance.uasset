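; BP_WMInstance is a central UI hub that exposes events for the main menu, info widgets, goal displays and a cutscene.
; Menu and cutscene set UI-only input, with the cutscene playing a sound and removing its widget after a fixed 59-second delay.
; AI, object and CCTV events forward to widget references assigned outside this graph.
; Four goal events each spawn a new UI_Goals, with the last three advancing CurrentGoalIndex.
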(event `ShowMainMenu`
  (bind _returnvalue (`GameplayStatics.GetPlayerController` 0))
  (`/Engine/EditorBlueprintResources/StandardMacros.IsValid` (`self.MainMenu`)
    (:`Is Valid`
      _)
    (:`Is Not Valid`
      (bind _returnvalue_2 (`|CreateWidget` "/Game/2_BP/BP_UI/UI_MainMenu.UI_MainMenu_C"))
      (bind _output_get (set `self.MainMenu` _returnvalue_2))))
  (`UserWidget.AddToViewport` _output_get 0)
  (`WidgetBlueprintLibrary.SetInputMode_UIOnlyEx` _returnvalue _output_get)
  (set `PlayerController.bShowMouseCursor` true _returnvalue))

(event `Show AI Data`
  (params (Num_AI :type String))
  (`/Game/2_BP/BP_UI/UI_HackedAIInfo.Get AI Data` (`self.CurrentAIWidget`) Num_AI))

(event `Show Object Data`
  (params (`Num Object` :type String))
  (`/Game/2_BP/BP_UI/UI_HackedObjectInfo.Get Object Data` (`self.CurrentObjectWidget`) `Num Object`))

(event `Show CCTV`
  (`/Game/2_BP/BP_UI/UI_HackedObjectInfo.Get CCTV Data` (`self.CurrentObjectWidget`)))

(event `EventUI_1st`
  (bind _returnvalue (`|CreateWidget` "/Game/2_BP/BP_UI/UI_Goals.UI_Goals_C"))
  (bind _output_get (set `self.CurrentGoalWidget` _returnvalue))
  (`/Game/2_BP/BP_UI/UI_Goals.Goal_1st` _output_get)
  (`UserWidget.AddToViewport` _output_get 0))

(event `EventUI_2nd`
  (`/Engine/EditorBlueprintResources/StandardMacros.IncrementInt` (`self.CurrentGoalIndex`)
    (:`  `
      (bind _returnvalue (`|CreateWidget` "/Game/2_BP/BP_UI/UI_Goals.UI_Goals_C"))
      (bind _output_get (set `self.CurrentGoalWidget` _returnvalue))
      (`/Game/2_BP/BP_UI/UI_Goals.Goal_2nd` _output_get)
      (`UserWidget.AddToViewport` _output_get 0))))

(event `EventUI_3rd`
  (`/Engine/EditorBlueprintResources/StandardMacros.IncrementInt` (`self.CurrentGoalIndex`)
    (:`  `
      (bind _returnvalue (`|CreateWidget` "/Game/2_BP/BP_UI/UI_Goals.UI_Goals_C"))
      (bind _output_get (set `self.CurrentGoalWidget` _returnvalue))
      (`/Game/2_BP/BP_UI/UI_Goals.Goal_3rd` _output_get)
      (`UserWidget.AddToViewport` _output_get 0))))

(event `EventUI_4th`
  (`/Engine/EditorBlueprintResources/StandardMacros.IncrementInt` (`self.CurrentGoalIndex`)
    (:`  `
      (bind _returnvalue (`|CreateWidget` "/Game/2_BP/BP_UI/UI_Goals.UI_Goals_C"))
      (bind _output_get (set `self.CurrentGoalWidget` _returnvalue))
      (`/Game/2_BP/BP_UI/UI_Goals.Goal_4th` _output_get)
      (`UserWidget.AddToViewport` _output_get 0))))

(event `CutScene`
  (bind _returnvalue (`GameplayStatics.GetPlayerController` 0))
  (bind _returnvalue_2 (`|CreateWidget` "/Game/2_BP/BP_UI/UI_CutScene.UI_CutScene_C"))
  (`UserWidget.AddToViewport` _returnvalue_2 0)
  (`WidgetBlueprintLibrary.SetInputMode_UIOnlyEx` _returnvalue _returnvalue_2)
  (set `PlayerController.bShowMouseCursor` false _returnvalue)
  (`GameplayStatics.PlaySound2D` "/Game/Movies/CutScene.CutScene" 1.0 1.0 0.0 null null)
  (`KismetSystemLibrary.Delay` 59.0)
  (`Widget.RemoveFromParent` _returnvalue_2))