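; Player character Blueprint for a shooter with hacking, handling armed aiming, firing, traversal and interaction UI.
; Shooting unzoomed triggers a temporary zoom that Tick reverts after a timer.
; While right-click aiming, a sphere's screen projection sets direction flags that Tick turns into pitch and yaw adjustments.
; Climb and vault play motion-warped montages in Flying mode without collision, while interaction events show hacking widgets for CCTVs and objects.
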(event `self.ReceiveTick`
  (params (DeltaSeconds :type "Float (single-precision)"))
  (bind _aimadjust (`self.AimAdjust`))
  (set `self.CurrentZoomTime` (+ DeltaSeconds (`self.CurrentZoomTime`)))
  (`|ExecutionSequence`
    (:`then_0`
      (if (and (`self.Shooting`) (> (`self.CurrentZoomTime`) (`self.ZoomTimeFlag`)))
        (`self.ZoomOut`)
        (set `self.Shooting` false)))
    (:`then_1`
      (if (`self.isUpperAim`)
        (set `self.PitchAd` (* (- (`self.PitchAd`) -0.6) _aimadjust))
        (if (`self.isLefterAim`) :!label _label
          (set `self.YawAd` (- (`self.YawAd`) 0.4))
          (elif (`self.isRighterAim`)
            (set `self.YawAd` (- (`self.YawAd`) -0.4))))
        (elif (`self.isBelowAim`)
          (set `self.PitchAd` (* (- (`self.PitchAd`) 0.6) _aimadjust))
          (goto _label))))
    (:`then_2`
      (if (`self.isRifle`)
        (set `self.M416BodyLoc` (`SceneComponent.GetSocketLocation` (`self.M416`) "gun_body"))))))

(event `self.ReceiveBeginPlay`
  (bind _asbp_wminstance (cast `/Game/2_BP/BP_System/BP_WMInstance` (`GameplayStatics.GetGameInstance`)))
  (set `WM_Instance.Player` self _asbp_wminstance)
  (bind _returnvalue (`|CreateWidget` "/Game/2_BP/BP_UI/UI_Player.UI_Player_C"))
  (`UserWidget.AddToViewport` _returnvalue 0)
  (bind _returnvalue_2 (`|CreateWidget` "/Game/2_BP/BP_UI/UI_HackedObjectInfo.UI_HackedObjectInfo_C"))
  (set `self.UI HackedObject` _returnvalue_2)
  (bind _returnvalue_3 (`|CreateWidget` "/Game/2_BP/BP_UI/UI_HackedCCTVInfo.UI_HackedCCTVInfo_C"))
  (set `self.UI HackedCCTV` _returnvalue_3)
  (set `self.ABP_Aiden` (`SkeletalMeshComponent.GetAnimInstance` (`self.Mesh`))))

(event `self.ReceivePossessed`
  (params (NewController :type "Controller Object Reference"))
  (set `self.IsPossessing` true))

(event `self.ReceiveUnpossessed`
  (params (OldController :type "Controller Object Reference"))
  (set `self.IsPossessing` false))

(event `EnhancedInput|/Game/6_MISC/Input/Actions/IA_MouseRightClick`
  (params (ActionValue :type Boolean) (ElapsedSeconds :type "Float (double-precision)") (TriggeredSeconds :type "Float (double-precision)") (InputAction :type "InputAction Object Reference" :default "/Game/6_MISC/Input/Actions/IA_MouseRightClick.IA_MouseRightClick"))
  (bind _returnvalue_x (`KismetMathLibrary.BreakVector2D` (`WidgetLayoutLibrary.GetViewportSize`)))
  (bind (_returnvalue_x_2 _returnvalue_y) (`KismetMathLibrary.BreakVector2D` (`WidgetLayoutLibrary.GetViewportSize`)))
  (bind _isarmed (`self.isArmed`))
  (bind _returnvalue (/ _returnvalue_x 2.0))
  (bind _returnvalue_2 (/ _returnvalue_y 2.0))
  (bind (_screenposition _returnvalue_3) (`GameplayStatics.ProjectWorldToScreen` (`GameplayStatics.GetPlayerController` 0) (`SceneComponent.K2_GetComponentLocation` (`self.SphereForAim`))))
  (:`Triggered`
    (if _isarmed
      (`self.ZoomIn`)
      (if _returnvalue_3
        (bind _output_get (set `self.AimPosition` _screenposition))
        (bind _returnvalue_4 (`KismetMathLibrary.FTrunc` (`.Y` (`KismetMathLibrary.BreakVector2D` _output_get))))
        (set `self.AimAdjust` (`KismetMathLibrary.FClamp` (/ (`KismetMathLibrary.Abs` (- _returnvalue_y _returnvalue_4)) 4.0)))
        (if (> (`KismetMathLibrary.Abs` (- _returnvalue_2 (`.Y` (`KismetMathLibrary.BreakVector2D` _output_get)))) 30.0)
          (if (> _returnvalue_4 (`KismetMathLibrary.FTrunc` _returnvalue_2))
            (set `self.isUpperAim` true)
            (set `self.isBelowAim` false)
            (else
              (set `self.isBelowAim` true)
              (set `self.isUpperAim` false)))
          (bind _output_get_2 (set `self.AimPosition` _screenposition))
          (if (> (`KismetMathLibrary.Abs` (- _returnvalue (`KismetMathLibrary.BreakVector2D` _output_get_2))) 50.0)
            (if (> (`KismetMathLibrary.FTrunc` (`KismetMathLibrary.BreakVector2D` _output_get_2)) (`KismetMathLibrary.FTrunc` _returnvalue))
              (set `self.isLefterAim` false)
              (set `self.isRighterAim` true)
              (else
                (set `self.isLefterAim` true)
                (set `self.isRighterAim` false)))
            (else
              (set `self.isLefterAim` false)
              (set `self.isRighterAim` false)))
          (else
            (set `self.isBelowAim` false)
            (set `self.isUpperAim` false))))))
  (:`Completed`
    (if _isarmed
      (`self.ZoomOut`)
      (set `self.isUpperAim` false)
      (set `self.isBelowAim` false)
      (set `self.isLefterAim` false)
      (set `self.isRighterAim` false))))

(event `EnhancedInput|/Game/6_MISC/Input/Actions/IA_Interaction`
  (params (ActionValue :type Boolean) (ElapsedSeconds :type "Float (double-precision)") (TriggeredSeconds :type "Float (double-precision)") (InputAction :type "InputAction Object Reference" :default "/Game/6_MISC/Input/Actions/IA_Interaction.IA_Interaction"))
  (bind _interactable_cctv (`self.Interactable CCTV`))
  (:`Triggered`
    (`self.InteractStart_1Sec`)
    (if (`KismetSystemLibrary.IsValid` _interactable_cctv) :!label _label_2
      (message `/Game/2_BP/BPI_HackableEvents.UpdateHackingProgress` _interactable_cctv (`self.InteractionTime`))))
  (:`Started`
    (`self.InteractionSinglePress`))
  (:`Completed`
    (`self.InteractEnd_1Sec`)
    (goto _label_2)))

(event `self.ClimbMotionWarp`
  (bind (_startpos_x _startpos_y _startpos_z) (`KismetMathLibrary.BreakVector` (`self.StartPos`)))
  (bind (_wallpos_x _wallpos_y) (`KismetMathLibrary.BreakVector` (`self.WallPos`)))
  ;[1 1 1] Climb Motion 정의
  (if (`self.canClimb`)
    (`CharacterMovementComponent.SetMovementMode` (`self.CharacterMovement`) "MOVE_Flying" 0)
    (`self.SetActorEnableCollision` false)
    (`MotionWarpingComponent.AddOrUpdateWarpTargetFromTransform` (`self.MotionWraping`) "attachedMotion" (`KismetMathLibrary.MakeTransform` (`KismetMathLibrary.MakeVector` _wallpos_x _wallpos_y _startpos_z)))
    (`|PlayMontage` (`self.Mesh`) "/Game/4_SK/Aiden/Montage/Braced_Hang_To_Crouch_Montage.Braced_Hang_To_Crouch_Montage" 1.5
      (:`OnCompleted`
        (`CharacterMovementComponent.SetMovementMode` (`self.CharacterMovement`) "MOVE_Walking" 0)
        (`self.SetActorEnableCollision` true)
        (`self.EnableInput` (`GameplayStatics.GetPlayerController` 0))))))

(event `EnhancedInput|/Game/6_MISC/Input/Actions/IA_MouseLeftClick`
  (params (ActionValue :type Boolean) (ElapsedSeconds :type "Float (double-precision)") (TriggeredSeconds :type "Float (double-precision)") (InputAction :type "InputAction Object Reference" :default "/Game/6_MISC/Input/Actions/IA_MouseLeftClick.IA_MouseLeftClick"))
  (:`Triggered`
    (if (`self.isZooming`) :!label _label_3
      (`self.Shoot`)
      (message `/Game/2_BP/Recoil.getRecoil` (`self.ABP_Aiden`))
      (else
        (`self.ZoomIn`)
        (set `self.CurrentZoomTime` 0.0)
        (set `self.Shooting` true)
        (`self.Shoot`)
        (set `self.isZooming` false))))
  (:`Started`
    (goto _label_3)))

(event `self.PlayStopMontage`
  (if (not (`self.isZooming`))
    (`self.PlayAnimMontage` null)))

(event `self.PlayShootMontage`)

(event `self.VaultMotionWarp`
  ;[1 1 1] Vault Motion 정의
  (`CharacterMovementComponent.SetMovementMode` (`self.CharacterMovement`) "MOVE_Flying" 0)
  (`self.SetActorEnableCollision` false)
  (`MotionWarpingComponent.AddOrUpdateWarpTargetFromTransform` (`self.MotionWraping`) "JumpPos" (`KismetMathLibrary.MakeTransform` (`self.StartPos`) (`self.K2_GetActorRotation`)))
  (`MotionWarpingComponent.AddOrUpdateWarpTargetFromTransform` (`self.MotionWraping`) "StandPos" (`KismetMathLibrary.MakeTransform` (`self.LastPos`)))
  (`|PlayMontage` (`self.Mesh`) "/Game/4_SK/Aiden/Montage/Jumping_Down_Montage.Jumping_Down_Montage" 1.5
    (:`OnCompleted`
      (`CharacterMovementComponent.SetMovementMode` (`self.CharacterMovement`) "MOVE_Walking" 0)
      (`self.SetActorEnableCollision` true)
      (`self.EnableInput` (`GameplayStatics.GetPlayerController` 0)))))

(event `EnhancedInput|/Game/6_MISC/Input/Actions/IA_ChangeGun`
  (params (ActionValue :type "Vector2D Structure") (ElapsedSeconds :type "Float (double-precision)") (TriggeredSeconds :type "Float (double-precision)") (InputAction :type "InputAction Object Reference" :default "/Game/6_MISC/Input/Actions/IA_ChangeGun.IA_ChangeGun"))
  (:`Started`
    (`self.ChangeGun`)))

(event `self.OnInteractionCCTV`
  (params (ContactActor :type "HitResult Structure"))
  (bind _asbp_cctv_hacked (cast `/Game/2_BP/BP_CCTV_Hacked` (`.HitActor` (`GameplayStatics.BreakHitResult` ContactActor))))
  (set `self.Interactable CCTV` _asbp_cctv_hacked)
  (`UserWidget.AddToViewport` (`self.UI HackedCCTV`) 0))

(event `self.EndInteraction`
  (`|ExecutionSequence`
    (:`then_0`
      (`Widget.RemoveFromParent` (`self.UI HackedCCTV`)))
    (:`then_1`
      (`Widget.RemoveFromParent` (`self.UI HackedObject`)))))

(event `self.OnInteractionObject`
  (params (ContactActor :type "HitResult Structure"))
  (bind _ui_hackedobject (`self.UI HackedObject`))
  (bind _ashackable_actor (cast `HackableActor` (`.HitActor` (`GameplayStatics.BreakHitResult` ContactActor))))
  (bind _output_get (set `self.Interactable Object` _ashackable_actor))
  (`/Game/2_BP/BP_UI/UI_HackedObjectInfo.Get Object Data` _ui_hackedobject (`HackableActor.Object_Num` _output_get))
  (`UserWidget.AddToViewport` _ui_hackedobject 0))

(fn `UserConstructionScript`)