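; BP_CCTV_2 is a controllable CCTV camera that can look around, interact, show hacking progress and return control to the player.
; Look input drives controller yaw and inverted pitch, and interaction input forwards to single-press and one-second hold functions defined outside these graphs.
; The back action calls Back2Player with the player stored in BP_WMInstance.
; Targeting reveals the interactable widget, whose progress bar uses a dynamic material parameter for hacking progress.
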(event `EnhancedInput|/Game/6_MISC/Input/Actions/IA_Look`
  (params (ActionValue :type "Vector2D Structure") (ElapsedSeconds :type "Float (double-precision)") (TriggeredSeconds :type "Float (double-precision)") (InputAction :type "InputAction Object Reference" :default "/Game/6_MISC/Input/Actions/IA_Look.IA_Look"))
  (:`Triggered`
    (`self.AddControllerYawInput` ActionValue_X)
    (`self.AddControllerPitchInput` (* ActionValue_Y -1.0))))

(event `EnhancedInput|/Game/6_MISC/Input/Actions/IA_Interaction`
  (params (ActionValue :type Boolean) (ElapsedSeconds :type "Float (double-precision)") (TriggeredSeconds :type "Float (double-precision)") (InputAction :type "InputAction Object Reference" :default "/Game/6_MISC/Input/Actions/IA_Interaction.IA_Interaction"))
  (:`Triggered`
    (`self.InteractStart_1Sec`))
  (:`Started`
    (`self.InteractionSinglePress`))
  (:`Completed`
    (`self.InteractEnd_1Sec`)))

(event `EnhancedInput|/Game/6_MISC/Input/Actions/IA_Back2Player`
  (params (ActionValue :type Boolean) (ElapsedSeconds :type "Float (double-precision)") (TriggeredSeconds :type "Float (double-precision)") (InputAction :type "InputAction Object Reference" :default "/Game/6_MISC/Input/Actions/IA_Back2Player.IA_Back2Player"))
  (:`Started`
    (bind _asbp_wminstance (cast `/Game/2_BP/BP_System/BP_WMInstance` (`GameplayStatics.GetGameInstance`)))
    (`self.Back2Player` (`WM_Instance.Player` _asbp_wminstance) (`GameplayStatics.GetPlayerController` 0))))

(event `/Game/2_BP/BPI_HackableEvents.UpdateHackingProgress`
  (params (`Progress Value` :type "Float (double-precision)"))
  (bind _asui_focused_interactable_actor (cast `/Game/2_BP/BP_UI/UI_FocusedInteractableActor` (`WidgetComponent.GetUserWidgetObject` (`self.Interactable Widget`))))
  (bind _progressbar (`/Game/2_BP/BP_UI/UI_FocusedInteractableActor.ProgressBar` _asui_focused_interactable_actor))
  (bind _returnvalue (`Image.GetDynamicMaterial` _progressbar))
  (`Image.SetBrushFromMaterial` _progressbar _returnvalue)
  (`MaterialInstanceDynamic.SetScalarParameterValue` _returnvalue "Progress" `Progress Value`))

(event `/Game/2_BP/BPI_HackableEvents.EventObjectTageted`
  (`SceneComponent.SetVisibility` (`self.Interactable Widget`) true false))

(fn `UserConstructionScript`)